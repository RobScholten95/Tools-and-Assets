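; Actor that lays out a row of static meshes along a referenced spline path, like linked carts.
; The construction script creates a component per mesh in Objects and stacks offsets from each mesh's Y bounds.
; UpdateCart places and rotates each mesh at its offset plus DistanceAlongSpline, rerunning on Tick while enabled.
; BeginPlay optionally attaches particle effects at a named socket; Tick handles FX pausing and array reversal.
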(event `self.ReceiveTick`
  (params (DeltaSeconds :type "Float (single-precision)"))
  ;[1 1 1] TICK
  (`|ExecutionSequence`
    (:`then_0`
      (if (`self.Enabled`)
        (`self.UpdateCart`)))
    (:`then_1`
      (if (`self.PausedFX`)
        (`ActorComponent.Deactivate` (`self.ParticleSystemOUT`))))
    (:`then_2`
      (if (`self.Objects Reversed`)
        (`self.Reverse Objects`)))))

(event `Reverse Objects`
  ;[1 1 1] REVERSING THE OBJECTS
  (`KismetArrayLibrary.Array_Reverse` (`self.Objects`)))

(event `self.ReceiveBeginPlay`
  ;[1 1 1] BEGINPLAY
  (if (`self.Enabled`)
    (if (`self.FX Enabled`)
      (`self.SpawnFX`))))

(event `UpdateCart`
  (bind _path (`/Game/ObjectAlongSplineTool/Spline/BP_SplinePath.Path` (`self.Spline Path to Follow`)))
  ;[1 1 1] UPDATE CART EVENT
  (for (_array_element _array_index) (`self.StaticMeshes`)
    (bind _returnvalue (/ (+ (`|GetArrayItem` (`self.ObjectOffsetY`) _array_index) (`self.Distance along Spline`)) (`self.ObjectOffsetDivider`)))
    (bind _returnvalue_location (`KismetMathLibrary.BreakTransform` (`KismetMathLibrary.MakeTransform` (+ (`SplineComponent.GetLocationAtDistanceAlongSpline` _path _returnvalue "World") (`KismetMathLibrary.MakeVector` 0.0 0.0 (`self.ObjectOffsetZ`))))))
    (`SceneComponent.K2_SetWorldLocation` _array_element _returnvalue_location false false)
    (`SceneComponent.K2_SetWorldRotation` _array_element (`KismetMathLibrary.ComposeRotators` (`SplineComponent.GetRotationAtDistanceAlongSpline` _path _returnvalue "World") (`self.Object Rotation`)) false false)))

(event `SpawnFX`
  ;[1 1 1] SPAWNING PARTICLE EFFECTS ON SOCKETS
  (for _array_element (`self.StaticMeshes`)
    (bind _returnvalue (`StaticMesh.FindSocket` (`StaticMeshComponent.StaticMesh` _array_element) (`self.SocketName1`)))
    (`/Engine/EditorBlueprintResources/StandardMacros.IsValid` _returnvalue
      (:`Is Valid`
        (bind _returnvalue_2 (`NiagaraFunctionLibrary.SpawnSystemAttached` (`self.Particle System`) _array_element "None" (`StaticMeshSocket.RelativeLocation` _returnvalue) (struct) "KeepRelativeOffset" false true "AutoRelease"))
        (set `self.ParticleSystemOUT` _returnvalue_2))
      (:`Is Not Valid`
        (`KismetSystemLibrary.PrintString` "Socket 1 is invalid")))))

(fn `UserConstructionScript`
  ;[1 1 1] ORIGINAL
  (`|ExecutionSequence`
    (:`then_0`
      (`KismetArrayLibrary.Array_Clear` (`self.StaticMeshes`))
      (`KismetArrayLibrary.Array_Clear` (`self.ObjectOffsetY`))
      (for _array_element (`self.Objects`)
        (bind _y (.y (`.BoxExtent` (`KismetMathLibrary.BreakBoxSphereBounds` (`StaticMesh.GetBounds` _array_element)))))
        (`KismetArrayLibrary.Array_Add` (`self.ObjectOffsetY`) (+ _y (.y (`self.ObjectOffsetVector`))))
        (set `self.ObjectOffsetVector` (`KismetMathLibrary.MakeVector` 0.0 (+ (.y (`self.ObjectOffsetVector`)) (* _y 2.0))))
        (bind _returnvalue (`AddComponent|NODE_AddStaticMeshComponent-7`))
        (`StaticMeshComponent.SetStaticMesh` _returnvalue _array_element)
        (`KismetArrayLibrary.Array_Add` (`self.StaticMeshes`) _returnvalue)))
    (:`then_1`
      (`self.UpdateCart`))))