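; Spline path actor that, when MeshEnabled is on, builds visible geometry along its Path spline in the Construction Script.
; A line pass adds one Y-forward spline mesh per segment, bent to the local locations and tangents of neighboring points.
; A crossbar pass places scaled static meshes at SpacingAlongLine intervals, rotated to follow the spline.
; The Event Graph has no active logic, only empty events and an unconnected copy of the line loop.
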(event `self.ReceiveBeginPlay`
  ;[1 1 1] Comment
)

(fn `UserConstructionScript`
  (bind _path (`self.Path`))
  (bind _path_2 (`self.Path`))
  (if (`self.Mesh Enabled`)
    (`|ExecutionSequence`
      (:`then_0`
        ;[1 1 1] Line
        (for _index (range (+ (- (`SplineComponent.GetNumberOfSplinePoints` (`self.Path`)) 2) 1))
          (bind _returnvalue (`AddComponent|NODE_AddSplineMeshComponent-8` :`RelativeTransform` (`KismetMathLibrary.MakeTransform` (0.0 0.0 0.0))))
          (`SplineMeshComponent.SetForwardAxis` _returnvalue "Y" true)
          (bind (_location _tangent) (`SplineComponent.GetLocationAndTangentAtSplinePoint` _path _index "Local"))
          (bind (_location_2 _tangent_2) (`SplineComponent.GetLocationAndTangentAtSplinePoint` _path (+ _index 1) "Local"))
          (`SplineMeshComponent.SetStartAndEnd` _returnvalue _location _tangent _location_2 _tangent_2 true)))
      (:`then_1`
        ;[1 1 1] Crossbars
        (for _index_2 (range (+ (`.ReturnValue` (`KismetMathLibrary.FMod` (`SplineComponent.GetSplineLength` (`self.Path`)) (`self.Spacing along line`))) 1))
          (bind _returnvalue_2 (* _index_2 (`self.Spacing along line`)))
          (bind _returnvalue_3 (`AddComponent|NODE_AddStaticMeshComponent-15` :`RelativeTransform` (`KismetMathLibrary.MakeTransform` (`SplineComponent.GetLocationAtDistanceAlongSpline` _path_2 _returnvalue_2 "Local") (`SplineComponent.GetRotationAtDistanceAlongSpline` _path_2 _returnvalue_2 "Local") (`self.Scale Crossbars`))))
          (`StaticMeshComponent.SetStaticMesh` _returnvalue_3 (`self.Static Mesh`))
          (`PrimitiveComponent.SetMaterial` _returnvalue_3 0 null))))))