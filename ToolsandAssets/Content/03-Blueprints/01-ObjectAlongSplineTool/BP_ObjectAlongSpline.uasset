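; Actor that lines up a list of static meshes along a spline path and moves them along it as a train, with optional attached particle effects.
; Construction script creates a component per mesh and stacks offsets from each mesh's Y bounds for spacing.
; A speed-scaled timeline drives distance over a hardcoded length, and Tick repositions and rotates each mesh on the spline.
; Niagara effects attach to meshes with the named socket, only while the valid-socket debug flag is on.
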(event `self.ReceiveBeginPlay`
  ;[1 1 1] BeginPlay
  (if (`self.Object Enabled`)
    (`|ExecutionSequence`
      (:`then_0`
        (`self.SpawnFX`))
      (:`then_1`
        (`self.Set Speed`)))))

(event `self.ReceiveTick`
  (params (DeltaSeconds :type "Float (single-precision)"))
  ;[1 1 1] Tick
  (if (`self.Object Enabled`)
    (`self.UpdateCart`)))

(event `UpdateCart`
  (bind _path (`/Game/03-Blueprints/01-ObjectAlongSplineTool/BP_Spline.Path` (`self.Path`)))
  ;[1 1 1] UPDATE CART EVENT
  (for (_array_element _array_index) (`self.StaticMeshes`)
    (bind _returnvalue (/ (+ (`|GetArrayItem` (`self.ObjectY`) _array_index) (`self.Distance along Spline`)) (`self.DivideOffset`)))
    (bind _returnvalue_location (`KismetMathLibrary.BreakTransform` (`KismetMathLibrary.MakeTransform` (+ (`SplineComponent.GetLocationAtDistanceAlongSpline` _path _returnvalue "World") (`KismetMathLibrary.MakeVector` 0.0 0.0 (`self.Z Offset`))))))
    (`SceneComponent.K2_SetWorldLocation` _array_element _returnvalue_location false false)
    (`SceneComponent.K2_SetWorldRotation` _array_element (`KismetMathLibrary.ComposeRotators` (`SplineComponent.GetRotationAtDistanceAlongSpline` _path _returnvalue "World") (`self.Rotation Object`)) false false)
    (`SceneComponent.SetWorldScale3D` _array_element (1.0 1.0 1.0))
    (bind _returnvalue_2 (`StaticMesh.FindSocket` (`StaticMeshComponent.StaticMesh` _array_element) (`self.Particle Socket Name`)))
    (`/Engine/EditorBlueprintResources/StandardMacros.IsValid` _returnvalue_2
      (:`Is Valid`
        (bind _relativelocation (`StaticMeshSocket.RelativeLocation` _returnvalue_2))
        (`SceneComponent.K2_SetRelativeLocation` (`self.ParticleFXOUT`) _relativelocation false false)
        (`KismetSystemLibrary.PrintString` (`KismetStringLibrary.Conv_VectorToString` _relativelocation) true true (struct :`R` 1.0 :`G` 0.193359 :`A` 1.0) 502.0)))))

(event `SpawnFX`
  ;[1 1 1] Spawn the ParticleSystem
  (if (`self.Spawn Particlesystem`)
    (for _array_element (`self.StaticMeshes`)
      (`/Engine/EditorBlueprintResources/StandardMacros.IsValid` (`StaticMesh.FindSocket` (`StaticMeshComponent.StaticMesh` _array_element) (`self.Particle Socket Name`))
        (:`Is Valid`
          ;;[1 1 1] Debug when socket is invalid
          (if (`self.Enable Debug - Particlesystems Sockets valid?`)
            (`KismetSystemLibrary.PrintString` (`KismetStringLibrary.Concat_StrStr` (`KismetSystemLibrary.GetObjectName` (`StaticMeshComponent.StaticMesh` _array_element)) " in " (`KismetSystemLibrary.GetDisplayName` self) " has a valid socket!") true true (struct :`G` 1.0 :`B` 0.040609 :`A` 1.0) (`self.Debug Durations`))
            (bind _returnvalue (`NiagaraFunctionLibrary.SpawnSystemAttached` (`self.ParticleSystem`) _array_element "None" (0.0 0.0 0.0) (struct) "KeepRelativeOffset" false true "ManualRelease" false))
            (set `self.ParticleFXOUT` _returnvalue)))
        (:`Is Not Valid`
          ;;[1 1 1] Debug when socket is invalid
          (if (`self.Enable Debug - Particlesystems Sockets valid?`)
            (`KismetSystemLibrary.PrintString` (`KismetStringLibrary.Concat_StrStr` (`KismetSystemLibrary.GetObjectName` (`StaticMeshComponent.StaticMesh` _array_element)) " in " (`KismetSystemLibrary.GetDisplayName` self) " does not have a valid socket!") true true (struct :`R` 1.0 :`G` 0.773574 :`A` 1.0) (`self.Debug Durations`))))))
    (else
      ;;[1 1 1] Debug when not enabled ParticleSystems
      (if (`self.Enable Debug - Particlesystems enabled?`)
        (`KismetSystemLibrary.PrintString` (`KismetStringLibrary.Concat_StrStr` "The particle system in " (`KismetSystemLibrary.GetDisplayName` self) " is turned off!") true true (struct :`R` 1.0 :`G` 0.411281 :`A` 1.0) (`self.Debug Durations`))))))

(event `Set Speed`
  ;[1 1 1] Set Speed
  (`TimelineComponent.SetPlayRate` (`self.TimelineDebug`) (`self.Speed`))
  (bind (_direction _movementtrack) (`Timeline|TimelineDebug` :!via `PlayFromStart`)
    (:`Update`
      (set `self.Distance along Spline` (* (- 1.0 _movementtrack) 21077.0)))))

(fn `NewFunction_0`)

(fn `UserConstructionScript`
  ;[1 1 1] ORIGINAL
  (`|ExecutionSequence`
    (:`then_0`
      (`KismetArrayLibrary.Array_Clear` (`self.StaticMeshes`))
      (`KismetArrayLibrary.Array_Clear` (`self.ObjectY`))
      (for _array_element (`self.Objects`)
        (bind _y (.y (`.BoxExtent` (`KismetMathLibrary.BreakBoxSphereBounds` (`StaticMesh.GetBounds` _array_element)))))
        (`KismetArrayLibrary.Array_Add` (`self.ObjectY`) (+ _y (.y (`self.Offset`))))
        (set `self.Offset` (`KismetMathLibrary.MakeVector` 0.0 (+ (.y (`self.Offset`)) (* _y 2.0))))
        (bind _returnvalue (`AddComponent|NODE_AddStaticMeshComponent-7`))
        (`StaticMeshComponent.SetStaticMesh` _returnvalue _array_element)
        (`KismetArrayLibrary.Array_Add` (`self.StaticMeshes`) _returnvalue)))
    (:`then_1`
      (`self.UpdateCart`))
    (:`then_2`
      (`KismetSystemLibrary.PrintString` "Hello"))))